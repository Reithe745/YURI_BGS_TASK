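; Base obstacle Blueprint that awards JumpingPoints when an interface-implementing actor overlaps its top collision box.
; BeginPlay splits the points into two digit meshes, zeroing the first when both match, and plays a timeline moving the display vertically.
; Tick spins the display.
; The overlap fires once, sends JumpedAboveMessage through BPI_JumpOverBlocksInteraction, hides the digits and runs fireworks for a short delay.
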(event `self.Top Collision Box.OnComponentBeginOverlap`
  (params (OverlappedComponent :type "PrimitiveComponent Object Reference") (OtherActor :type "Actor Object Reference") (OtherComp :type "PrimitiveComponent Object Reference") (OtherBodyIndex :type Integer) (bFromSweep :type Boolean) (SweepResult :type "HitResult Structure (by ref)"))
  (bind _fireworks (`self.Fireworks`))
  ;[1 1 1] Comunication through BPI system
  (if (`KismetSystemLibrary.DoesImplementInterface` OtherActor "/Game/MainAssets/Interfaces/BPI_JumpOverBlocksInteraction.BPI_JumpOverBlocksInteraction_C")
    (`/Engine/EditorBlueprintResources/StandardMacros.DoOnce` false
      (:`Completed`
        (message `/Game/MainAssets/Interfaces/BPI_JumpOverBlocksInteraction.Jumped Above` OtherActor (`self.Jumping Points`))
        ;;[1 0.4762 0] Particle system
        (`ActorComponent.Activate` _fireworks false)
        (`SceneComponent.SetHiddenInGame` (`self.First Number`) true false)
        (`SceneComponent.SetHiddenInGame` (`self.Second Number`) true false)
        (`KismetSystemLibrary.Delay` 2.0)
        (`ActorComponent.Deactivate` _fireworks)))))

(event `self.ReceiveBeginPlay`
  (bind (_initial_world_location_x _initial_world_location_y _initial_world_location_z) (`KismetMathLibrary.BreakVector` (`self.Initial world location`)))
  (`|ExecutionSequence`
    (:`then_0`
      ;[1 0 0.8006] Setup for points numbers explicit on the number components
      (bind _output_get (set `self.Points Number` (`KismetStringLibrary.Conv_IntToString` (`self.Jumping Points`))))
      (bind _output_get_2 (set `self.First digit` (`KismetStringLibrary.Left` _output_get 1)))
      (bind _output_get_3 (set `self.Second digit` (`KismetStringLibrary.Right` _output_get 1)))
      (if (`KismetStringLibrary.EqualEqual_StrStr` _output_get_3 _output_get_2)
        (set `self.First digit` "0"))
      (set `self.Initial world location` (`SceneComponent.K2_GetComponentLocation` (`self.PointDisplay`))))
    (:`then_1`
      ;[1 0.4405 0] Set assets numbers
      (`self.Set Mesh For Numbers` (`self.First digit`) (`self.First Number`)))
    (:`then_2`
      (`self.Set Mesh For Numbers` (`self.Second digit`) (`self.Second Number`)))
    (:`then_3`
      ;[0 1 0.3061] Number assets movement animation
      (bind (_direction _newtrack_0) (`Timeline|Rover`)
        (:`Update`
          (`SceneComponent.K2_SetWorldLocation` (`self.PointDisplay`) (`KismetMathLibrary.MakeVector` _initial_world_location_x _initial_world_location_y (`KismetMathLibrary.Lerp` _initial_world_location_z (+ _initial_world_location_z 20.0) _newtrack_0)) false false))))))

(event `self.ReceiveTick`
  (params (DeltaSeconds :type "Float (single-precision)"))
  ;[0 1 0.3061] Number assets movement animation
  (`SceneComponent.K2_AddLocalRotation` (`self.PointDisplay`) (`KismetMathLibrary.MakeRotator` 0.0 0.0 (* DeltaSeconds 100.0)) false false))

(fn `Set Mesh For Numbers`
  (params (Number :type String) (Asset :type "StaticMeshComponent Object Reference"))
  (`StaticMeshComponent.SetStaticMesh` Asset (select `int` (`KismetStringLibrary.Conv_StringToInt` Number) :`0` "/Game/Deko_MatrixDemo/City/Meshes/SM_Kit_Prop_Number_House_B00_N1.SM_Kit_Prop_Number_House_B00_N1" :`1` "/Game/Deko_MatrixDemo/City/Meshes/SM_Kit_Prop_Number_House_B01_N1.SM_Kit_Prop_Number_House_B01_N1" :`2` "/Game/Deko_MatrixDemo/City/Meshes/SM_Kit_Prop_Number_House_B02_N1.SM_Kit_Prop_Number_House_B02_N1" :`3` "/Game/Deko_MatrixDemo/City/Meshes/SM_Kit_Prop_Number_House_B03_N1.SM_Kit_Prop_Number_House_B03_N1" :`4` "/Game/Deko_MatrixDemo/City/Meshes/SM_Kit_Prop_Number_House_B04_N1.SM_Kit_Prop_Number_House_B04_N1" :`5` "/Game/Deko_MatrixDemo/City/Meshes/SM_Kit_Prop_Number_House_B05_N1.SM_Kit_Prop_Number_House_B05_N1" :`6` "/Game/Deko_MatrixDemo/City/Meshes/SM_Kit_Prop_Number_House_B06_N1.SM_Kit_Prop_Number_House_B06_N1" :`7` "/Game/Deko_MatrixDemo/City/Meshes/SM_Kit_Prop_Number_House_B07_N1.SM_Kit_Prop_Number_House_B07_N1" :`8` "/Game/Deko_MatrixDemo/City/Meshes/SM_Kit_Prop_Number_House_B08_N1.SM_Kit_Prop_Number_House_B08_N1" :`9` "/Game/Deko_MatrixDemo/City/Meshes/SM_Kit_Prop_Number_House_B09_N1.SM_Kit_Prop_Number_House_B09_N1" :!type "StaticMesh Object Reference")))

(fn `UserConstructionScript`)